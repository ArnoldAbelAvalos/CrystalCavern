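; BP_WinVolume is the level exit trigger in Crystal Cavern that completes the level when the player overlaps it.
; It blocks completion with an on-screen message while any BP_Crystal actors remain in the level.
; Otherwise it finds the current level in its LevelNames array and opens the next one, or prints a game-over message on the last level.
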(event `self.ReceiveActorBeginOverlap`
  (params (OtherActor :type "Actor Object Reference"))
  (cast `/Game/CrystalCavern/Blueprints/Pawns/BP_Player` OtherActor)
  (if (`self.AnyCrystalsRemaining`)
    (`KismetSystemLibrary.PrintString` "There are more crystals to collect")
    (else
      (`self.LevelComplete`))))

(fn `AnyCrystalsRemaining`
  (returns (ReturnValue :type Boolean))
  (bind _outactors (`GameplayStatics.GetAllActorsOfClass` "/Game/CrystalCavern/Blueprints/Actors/Collectables/BP_Crystal.BP_Crystal_C"))
  (return (> (`KismetArrayLibrary.Array_Length` _outactors) 0)))

(fn `IsLastLevel`
  (returns (ReturnValue :type Boolean) (NextLevelName :type Name))
  (bind _level_names (`self.Level Names`))
  (bind _returnvalue (`GameplayStatics.GetCurrentLevelName` true))
  (bind _returnvalue_2 (`KismetArrayLibrary.Array_Find` _level_names (`KismetStringLibrary.Conv_StringToName` _returnvalue)))
  (return (== _returnvalue_2 (`KismetArrayLibrary.Array_LastIndex` _level_names)) (`|GetArrayItem` (`self.Level Names`) (+ _returnvalue_2 1))))

(fn `LevelComplete`
  (bind (_returnvalue _nextlevelname) (`self.IsLastLevel`))
  (if _returnvalue
    (`KismetSystemLibrary.PrintString` "Game Over")
    (else
      (`GameplayStatics.OpenLevel` _nextlevelname))))

(fn `UserConstructionScript`)