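; BP_Cannon is an enemy cannon actor that automatically fires projectiles at a regular interval for as long as it runs.
; From BeginPlay, a self-repeating Delay on FireRate spawns a BP_Projectile at the Arrow component's world location and rotation.
; Each shot also restarts the CannonFire timeline, which slides the Cannon component along its relative Y axis to animate the barrel.
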(event `self.ReceiveBeginPlay`
  (`KismetSystemLibrary.Delay` (`self.FireRate`) :!label _label)
  (`|ExecutionSequence`
    (:`then_0`
      (`self.FireProjectile`)
      (goto _label))
    (:`then_1`
      (bind (_direction _cannonbarrellocation) (`Timeline|CannonFire` :!via `PlayFromStart`)
        (:`Update`
          (`self.AnimateCannon` _cannonbarrellocation))))))

(fn `AnimateCannon`
  (params (Location :type "Float (double-precision)"))
  (`SceneComponent.K2_SetRelativeLocation` (`self.Cannon`) (`KismetMathLibrary.MakeVector` 0.0 Location) false false))

(fn `FireProjectile`
  (bind _arrow (`self.Arrow`))
  (`|SpawnActorFromClass` "/Game/CrystalCavern/Blueprints/Actors/Porjectiles/BP_Projectile.BP_Projectile_C" (`KismetMathLibrary.MakeTransform` (`SceneComponent.K2_GetComponentLocation` _arrow) (`SceneComponent.K2_GetComponentRotation` _arrow)) "Undefined" "OverrideRootScale" null null))

(fn `UserConstructionScript`)