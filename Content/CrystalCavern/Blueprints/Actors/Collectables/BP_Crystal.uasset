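; BP_Crystal is a collectable crystal that flies into the player and vanishes when touched.
; Overlap of its sphere collision with BP_Player stores the starting location and scale, then plays the AlphaBlending timeline.
; Each update lerps the crystal toward the player pawn's current location, so it homes on a moving player, while shrinking it to zero scale.
; The actor destroys itself when the timeline finishes.
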(event `self.SphereCollision.OnComponentBeginOverlap`
  (params (OverlappedComponent :type "PrimitiveComponent Object Reference") (OtherActor :type "Actor Object Reference") (OtherComp :type "PrimitiveComponent Object Reference") (OtherBodyIndex :type Integer) (bFromSweep :type Boolean) (SweepResult :type "HitResult Structure (by ref)"))
  ;[1 1 1] On Player Overlap
  (cast `/Game/CrystalCavern/Blueprints/Pawns/BP_Player` OtherActor)
  (`self.StoreStartingValues`)
  (bind (_direction _alpha) (`Timeline|AlphaBlending`)
    (:`Update`
      (`self.UpdateCrystalLocationAndScale` _alpha))
    (:`Finished`
      (`self.K2_DestroyActor`))))

(fn `StoreStartingValues`
  (set `self.StartLocation` (`self.K2_GetActorLocation`))
  (set `self.StartScale` (`self.GetActorScale3D`)))

(fn `UpdateCrystalLocationAndScale`
  (params (Alpha :type "Float (double-precision)"))
  (`self.K2_SetActorLocation` (`KismetMathLibrary.VLerp` (`self.StartLocation`) (`self.K2_GetActorLocation` (`GameplayStatics.GetPlayerPawn` 0)) Alpha))
  (`self.SetActorScale3D` (`KismetMathLibrary.VLerp` (`self.StartScale`) (0.0 0.0 0.0) Alpha)))

(fn `UserConstructionScript`)