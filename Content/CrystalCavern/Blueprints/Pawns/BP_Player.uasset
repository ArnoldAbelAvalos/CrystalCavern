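; BP_Player is the player pawn, a physics sphere rolled by torque from movement input each tick.
; It fades the camera in on start; the first damage taken fades it out and reloads the current level, using the damage amount as fade and delay time.
; AdjustSpringArm sets the camera arm's length and world rotation, and the Quit action exits the game.
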(event `self.ReceiveBeginPlay`
  ;[1 1 1] Camera Fade on Start
  (`PlayerCameraManager.StartCameraFade` :`self` (`GameplayStatics.GetPlayerCameraManager` 0) :`FromAlpha` 1.0 :`Duration` 2.0))

(event `self.ReceiveTick`
  (params (DeltaSeconds :type "Float (single-precision)"))
  (bind _returnvalue (* DeltaSeconds (`self.Acceleration Multiplier`)))
  ;[1 1 1] Player Movement
  (`PrimitiveComponent.AddTorqueInRadians` (`self.Sphere`) (`KismetMathLibrary.MakeVector` (* _returnvalue (`self.GetInputAxisValue`)) (* _returnvalue (`self.GetInputAxisValue`))) "None" true))

(event `self.ReceiveAnyDamage`
  (params (Damage :type "Float (single-precision)") (DamageType :type "DamageType Object Reference") (InstigatedBy :type "Controller Object Reference") (DamageCauser :type "Actor Object Reference"))
  ;[1 1 1] Restart Level on Dmg Taken
  (`/Engine/EditorBlueprintResources/StandardMacros.DoOnce` false
    (:`Completed`
      (`PlayerCameraManager.StartCameraFade` :`self` (`GameplayStatics.GetPlayerCameraManager` 0) :`ToAlpha` 1.0 :`Duration` Damage :`bHoldWhenFinished` true)
      (`KismetSystemLibrary.Delay` Damage)
      (bind _returnvalue (`GameplayStatics.GetCurrentLevelName` true))
      (`GameplayStatics.OpenLevel` (`KismetStringLibrary.Conv_StringToName` _returnvalue)))))

(event `InputAction|Quit`
  (params (Key :type "Key Structure"))
  ;[1 1 1] Quit Game
  (:`Pressed`
    (`KismetSystemLibrary.QuitGame` null "Quit")))

(fn `AdjustSpringArm`
  (params (Distance :type "Float (double-precision)") (Rotation :type "Rotator Structure"))
  (bind _springarm (`self.SpringArm`))
  (set `SpringArmComponent.TargetArmLength` Distance _springarm)
  (`SceneComponent.K2_SetWorldRotation` _springarm Rotation false false))

(fn `UserConstructionScript`)